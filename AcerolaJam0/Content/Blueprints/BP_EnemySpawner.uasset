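; Enemy spawner actor that endlessly spawns BP_EnemyCharChild at its own transform, as either regular or boss enemies via the BossSpawner flag.
; Regular spawners start immediately, boss spawners after a timer; SpawnEnemy then re-calls itself through a Delay that shrinks to a clamped minimum.
; Each spawn receives the incrementing wave number, boss flag and HP, attack and speed values, which ScaleEnemyStats derives from player stats but is not called here.
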(event `self.ReceiveBeginPlay`
  (if (`self.Boss Spawner`)
    (`KismetSystemLibrary.K2_SetTimerDelegate` (delegate `Spawn Enemy`) (`self.Boss Timer`))
    (else
      (`self.Spawn Enemy`))))

(event `Spawn Enemy`
  (`|SpawnActorFromClass` "/Game/Blueprints/BP_EnemyCharChild.BP_EnemyCharChild_C" (`self.GetTransform`) "Undefined" "MultiplyWithRoot" null (`self.Current Wave`) (`self.Boss Spawner`) (`self.Variable To Player HP`) (`self.Variable To Player ATK`) (`self.Variable Speed`) null)
  (`/Engine/EditorBlueprintResources/StandardMacros.IncrementInt` (`self.Current Wave`)
    (:`  `
      (set `self.Boss Timer` (`KismetMathLibrary.FClamp` (- (`self.Boss Timer`) 90.0) 10.0 999.0))
      (if (`self.Boss Spawner`)
        (`KismetSystemLibrary.Delay` (`self.Boss Timer`))
        (else
          (bind _output_get (set `self.Spawn Timer` (`KismetMathLibrary.FClamp` (- (`self.Spawn Timer`) 6.0) 5.0 60.0)))
          (`KismetSystemLibrary.Delay` _output_get)))
      (`self.Spawn Enemy`))))

(event `Scale Enemy Stats`
  (bind (_hp _atk _roll_loop_speed) (message `/Game/Interface/ParentChar_INT.Return Stats` (`GameplayStatics.GetPlayerCharacter` 0)))
  (set `self.Variable To Player HP` (/ _hp 3))
  (set `self.Variable To Player ATK` (* _atk 2))
  (set `self.Variable Speed` (/ _roll_loop_speed 4.0)))

(fn `UserConstructionScript`)