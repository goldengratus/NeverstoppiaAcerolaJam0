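; BP_Projectile is an attack projectile for either player-controlled or enemy attackers, damaging characters of the opposing side.
; Construction sets initial speed and picks the player or enemy particle template; BeginPlay sets lifespan and initializes the attack component.
; Sphere overlaps identify targets through message calls, track hit actors to avoid repeats, then send damage without push.
; Non-Persistent projectiles die on damaging a character; non-Forever ones die on touching non-characters.
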(event `self.ReceiveBeginPlay`
  (bind _bp_atkcomponent (`self.BP_ATKComponent`))
  (`self.SetLifeSpan` (`self.In Lifespan`))
  (`/Game/Blueprints/BP_ATKComponent.Assign or Get Resource Bar` _bp_atkcomponent (`self.Widget`) (`self.Player Controlled?`))
  (`/Game/Blueprints/BP_ATKComponent.Update ATK` _bp_atkcomponent (`self.ATK-Value`)))

(event `self.Sphere1.OnComponentBeginOverlap`
  (params (OverlappedComponent :type "PrimitiveComponent Object Reference") (OtherActor :type "Actor Object Reference") (OtherComp :type "PrimitiveComponent Object Reference") (OtherBodyIndex :type Integer) (bFromSweep :type Boolean) (SweepResult :type "HitResult Structure (by ref)"))
  (bind _character_ (message `/Game/Interface/ParentChar_INT.Return is Character` OtherActor))
  (if _character_
    (bind _is_player (message `/Game/Interface/ParentChar_INT.Return is Player` OtherActor))
    (if (!= _is_player (`self.Player Controlled?`))
      (if (not (`KismetArrayLibrary.Array_Contains` (`self.Atked Array`)))
        (`KismetArrayLibrary.Array_AddUnique` (`self.Atked Array`) OtherActor)
        (message `/Game/Interface/ParentChar_INT.HP-Damage` OtherActor (`self.ATK-Value`) (0.0 0.0 0.0) (`self.Atker`))
        (`self.Hit Something`)
        (if (not (`self.Persistent?`))
          (`self.K2_DestroyActor`))))
    (elif (not (`self.Forever!`))
      (`self.K2_DestroyActor`))))

(fn `UserConstructionScript`
  (set `ProjectileMovementComponent.InitialSpeed` (`self.Initial Speed`) (`self.ProjectileMovement`))
  (`ParticleSystemComponent.SetTemplate` (`self.ProjectileSystem`) (select `bool` (`self.Player Controlled?`) :`false` (`self.Enemy System`) :`true` (`self.Player System`))))