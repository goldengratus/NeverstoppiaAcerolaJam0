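; Enemy character child Blueprint that picks one of five types on spawn by current wave and starts a thrust attack.
; Regular enemies roll a random type up to the wave, while bosses use the wave's type with boosted stats and a random super.
; SetEnemyType applies look, drop and stats adjusted by scaling variables.
; Boss death triggers victory on wave 4, otherwise a player super message and spawner stat scaling.
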(event `self.ReceiveBeginPlay`
  (`parent.ReceiveBeginPlay`)
  (`self.Change Enemy Type`)
  (`self.ThrustAttack`))

(event `Change Enemy Type`
  (switch `int` (`KismetMathLibrary.SelectInt` (`KismetMathLibrary.Clamp` (`self.Current Wave`) 0 4) (`KismetMathLibrary.RandomIntegerInRange` 0 (`KismetMathLibrary.Clamp` (`self.Current Wave`) 0 4)) (`self.BossType?`))
    (:`0`
      (`self.Set Enemy Type` (struct :`R` 0.848958 :`G` 0.008843 :`B` 0.148471 :`A` 1.0) (1.0 1.0 1.0) "NewEnumerator0" 3.0 1 1 "/Game/Mats/MI_Chars1.MI_Chars1"))
    (:`1`
      (`self.Set Enemy Type` (struct :`G` 1.0 :`B` 0.262087 :`A` 1.0) (0.6 0.6 0.6) "NewEnumerator2" 1.6 1 1 "/Game/Mats/MI_Chars2.MI_Chars2"))
    (:`2`
      (`self.Set Enemy Type` (struct :`R` 1.0 :`G` 0.924422 :`A` 1.0) (1.8 1.8 1.8) "NewEnumerator1" 2.5 2 2 "/Game/Mats/MI_Chars3.MI_Chars3"))
    (:`3`
      (`self.Set Enemy Type` (struct :`R` 0.016631 :`G` 0.121267 :`B` 1.0 :`A` 1.0) (1.4 1.4 1.4) "NewEnumerator4" 1.8 3 2 "/Game/Mats/MI_Chars6.MI_Chars6" (0.0 0.0 100.0)))
    (:`4`
      (`self.Set Enemy Type` (struct :`R` 0.335981 :`B` 1.0 :`A` 1.0) (2.0 2.0 2.0) "NewEnumerator3" 1.2 4 4 "/Game/Mats/MI_Chars4.MI_Chars4"))))

(event `self.Do Death THING`
  (bind _bosstype_ (`self.BossType?`))
  (`parent.Do Death THING`)
  (if (and (== (`self.Current Wave`) 4) _bosstype_)
    (message `/Game/Interface/GameInstance_INT.Victory!` (`GameplayStatics.GetGameInstance`))
    (elif _bosstype_
      (message `/Game/Interface/ParentChar_INT.Activate Super` (`GameplayStatics.GetPlayerCharacter` 0) (`self.Super Type`))
      (bind _outactors (`GameplayStatics.GetAllActorsOfClass` "/Game/Blueprints/BP_EnemySpawner.BP_EnemySpawner_C"))
      (for _array_element _outactors
        (`/Game/Blueprints/BP_EnemySpawner.Scale Enemy Stats` _array_element)))))

(fn `Set Enemy Type`
  (params (`HP COLOR` :type "LinearColor Structure") (NewScale3D :type "Vector Structure") (PowerUpToDrop :type "/Game/Enums/StatsEnum Enum" :default "NewEnumerator0") (`Roll Loop Speed` :type "Float (single-precision)") (`Value Added to HP` :type Integer) (ATK :type Integer) (Material :type "MaterialInterface Object Reference") (`Jump Power` :type "Vector Structure"))
  (bind _bosstype_ (`self.BossType?`))
  (set `self.HP COLOR` `HP COLOR`)
  (`self.SetActorScale3D` (* NewScale3D (select `bool` _bosstype_ :`false` 1.0 :`true` 2.0 :!type "Float (single-precision)")))
  (set `self.PowerUpToDrop` PowerUpToDrop)
  (set `self.Roll Loop Speed` (`KismetMathLibrary.FClamp` (- (* `Roll Loop Speed` (`KismetMathLibrary.SelectFloat` 0.5 1.0 _bosstype_)) (`self.variable speed`)) 0.1 9999.0))
  (`PrimitiveComponent.SetMaterial` (`self.Mesh`) 0 Material)
  (bind _current_hp_output (`self.Change HP` (+ (* `Value Added to HP` (`KismetMathLibrary.SelectInt` 10 1 _bosstype_)) (`self.Variable to Player ATK`))))
  (`self.Update Max HP` _current_hp_output)
  (set `self.ATK` (+ (* ATK (`KismetMathLibrary.SelectInt` 5 1 _bosstype_)) (`self.Variable to Player HP`)))
  (`self.Update Atk HUD`)
  (set `self.Jump Power` `Jump Power`)
  (if (`self.BossType?`)
    (bind _output_get (set `self.Super Type` (cast `/Game/Enums/SupersEnum` (`KismetMathLibrary.Conv_IntToByte` (`KismetMathLibrary.RandomInteger` (enumcount `/Game/Enums/SupersEnum`))))))
    (`/Game/Interface/ParentChar_INT.Activate Super` _output_get)))

(fn `UserConstructionScript`
  (`parent.UserConstructionScript`))