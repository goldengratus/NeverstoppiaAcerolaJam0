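; BP_LightningStorm is a lightning storm Blueprint, apparently an attack, that extends parent logic with hit-list resetting and adjustable spin.
; On BeginPlay it runs the parent logic, then binds a handler to HitSomething that clears AtkedArray whenever that event fires.
; A separate IncreaseRotation function steps up the RotatingMovement yaw rate by a fixed amount, though nothing in this file calls it.
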(event `self.ReceiveBeginPlay`
  (`parent.ReceiveBeginPlay`)
  (add `self.Hit Something` (delegate `Clear array`)))

(event `Clear array`
  (`KismetArrayLibrary.Array_Clear` (`self.Atked Array`)))

(fn `Increase Rotation`
  (bind _rotatingmovement (`self.RotatingMovement`))
  (bind (_rotationrate_roll _rotationrate_pitch _rotationrate_yaw) (`KismetMathLibrary.BreakRotator` (`RotatingMovementComponent.RotationRate` _rotatingmovement)))
  (set `RotatingMovementComponent.RotationRate` (`KismetMathLibrary.MakeRotator` 0.0 0.0 (+ _rotationrate_yaw 5.0)) _rotatingmovement))

(fn `UserConstructionScript`
  (`parent.UserConstructionScript`))