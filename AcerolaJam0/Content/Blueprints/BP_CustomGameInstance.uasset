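; Custom game instance that handles level restarts and the victory notification.
; RestartGame unpauses and calls RestartLevel, which waits a given delay, restores game-only input, sets a ResetGame flag and reopens the current level by name.
; The flag is exposed through a getter, so it can be read after the reload.
; Victory plays a 2D sound and changes the player character's menu message.
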(event `Restart Level`
  (params (Duration :type "Float (single-precision)"))
  (`KismetSystemLibrary.Delay` Duration)
  (`WidgetBlueprintLibrary.SetInputMode_GameOnly` (`GameplayStatics.GetPlayerController` 0))
  (set `self.Reset Game?` true)
  (bind _returnvalue (`GameplayStatics.GetCurrentLevelName` true))
  (`GameplayStatics.OpenLevel` (`KismetStringLibrary.Conv_StringToName` _returnvalue)))

(event `/Game/Interface/GameInstance_INT.Restart Game`
  (params (ResetDelay :type "Float (double-precision)"))
  (`GameplayStatics.SetGamePaused` false)
  (`self.Restart Level` ResetDelay))

(event `/Game/Interface/GameInstance_INT.Victory!`
  (`GameplayStatics.PlaySound2D` "/Game/MusicAndSound/victory.victory" 1.0 1.0 0.0 null null)
  (message `/Game/Interface/ParentChar_INT.Change Menu` (`GameplayStatics.GetPlayerCharacter` 0) "NewEnumerator2"))

(fn `Return Reset?`
  (returns (`Reset Game?` :type Boolean))
  (return (`self.Reset Game?`)))