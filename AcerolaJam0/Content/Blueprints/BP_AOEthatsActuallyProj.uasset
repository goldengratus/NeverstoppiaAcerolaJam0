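; Spawned magic-circle attack actor, named as an AOE that is actually a projectile, that lasts about ten seconds.
; On BeginPlay it runs the parent logic, then sets up its ATK component as non-player and applies its attack value.
; After a delay it deactivates the magic circle particle effect, and that system's finished event destroys the actor.
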(event `self.ReceiveBeginPlay`
  (bind _bp_atkcomponent1 (`self.BP_ATKComponent1`))
  (`parent.ReceiveBeginPlay`)
  (add `ParticleSystemComponent.OnSystemFinished` (`self.P_ky_magicCircle1`) (delegate `CustomEvent_0`))
  (`/Game/Blueprints/BP_ATKComponent.Assign or Get Resource Bar` _bp_atkcomponent1 (`self.ATK`) false)
  (`/Game/Blueprints/BP_ATKComponent.Update ATK` _bp_atkcomponent1 (`self.ATK-Value`))
  (`KismetSystemLibrary.Delay` 10.0)
  (`ActorComponent.Deactivate` (`self.P_ky_magicCircle1`)))

(event `CustomEvent_0`
  (params (PSystem :type "ParticleSystemComponent Object Reference"))
  (`self.K2_DestroyActor`))

(fn `UserConstructionScript`
  (`parent.UserConstructionScript`))