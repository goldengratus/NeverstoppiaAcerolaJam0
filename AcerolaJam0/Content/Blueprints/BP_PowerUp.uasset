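; BP_PowerUp is a collectible pickup that grants a typed power-up (HP, ATK, SPD, JUMP, SHOOT or VICTORY) to the player.
; On BeginPlay it picks a mesh by type, scales it in with a timeline, then enables collision and applies the type's material.
; On overlap, message calls confirm the player and grant the power-up once, then it plays particle and sound effects and destroys itself.
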(event `self.ReceiveBeginPlay`
  (`self.Set Mesh Powerup` (`self.PowerUpType`))
  (set `self.DefaultPowerUpScale` (`SceneComponent.K2_GetComponentScale` (`self.Cube`)))
  (bind (_direction _alpha) (`Timeline|TimelineToActivate`)
    (:`Update`
      (`SceneComponent.SetWorldScale3D` (`self.Cube`) (* (`self.DefaultPowerUpScale`) _alpha)))
    (:`Finished`
      (`PrimitiveComponent.SetCollisionEnabled` (`self.SphereCollision`) "QueryOnly")
      (bind _cube (`self.Cube`)
        (:`then`
          (`PrimitiveComponent.SetMaterial` _cube 0 (select `/Game/Enums/StatsEnum` (`self.PowerUpType`) :`NewEnumerator0` "/Game/Mats/MI_Chars1.MI_Chars1" :`NewEnumerator1` "/Game/Mats/MI_Chars3.MI_Chars3" :`NewEnumerator2` "/Game/Mats/MI_Chars2.MI_Chars2" :`NewEnumerator4` "/Game/Mats/MI_Chars6.MI_Chars6" :`NewEnumerator3` "/Game/Mats/MI_Chars4.MI_Chars4" :`NewEnumerator5` "/Game/Mats/MI_Chars.MI_Chars" :!type "MaterialInterface Object Reference")))
        (:`else`)))))

(event `Set Mesh Powerup`
  (params (MeshType :type "/Game/Enums/StatsEnum Enum" :default "NewEnumerator0"))
  (bind _output_get (set `self.Mesh Type` MeshType))
  (`StaticMeshComponent.SetStaticMesh` (`self.Cube`) (select `/Game/Enums/StatsEnum` _output_get :`NewEnumerator0` "/Game/StaticMeshes/Heart.Heart" :`NewEnumerator1` "/Game/StaticMeshes/swordpowerup.swordpowerup" :`NewEnumerator2` "/Game/StaticMeshes/SM_Boot.SM_Boot" :`NewEnumerator4` "/Game/StaticMeshes/jumppower.jumppower" :`NewEnumerator3` "/Game/StaticMeshes/SM_Bullet.SM_Bullet" :`NewEnumerator5` "/Game/StaticMeshes/SM_Victory.SM_Victory" :!type "StaticMesh Object Reference")))

(event `self.SphereCollision.OnComponentBeginOverlap`
  (params (OverlappedComponent :type "PrimitiveComponent Object Reference") (OtherActor :type "Actor Object Reference") (OtherComp :type "PrimitiveComponent Object Reference") (OtherBodyIndex :type Integer) (bFromSweep :type Boolean) (SweepResult :type "HitResult Structure (by ref)"))
  (bind _is_player (message `/Game/Interface/ParentChar_INT.Return is Player` OtherActor))
  (if _is_player
    (`/Engine/EditorBlueprintResources/StandardMacros.DoOnce` false
      (:`Completed`
        (message `/Game/Interface/ParentChar_INT.Give Power Up` OtherActor (`self.PowerUpType`))
        (`GameplayStatics.SpawnEmitterAtLocation` "/Game/FXVarietyPack/Particles/P_ky_hit1.P_ky_hit1" (`SceneComponent.K2_GetComponentLocation` (`self.Cube`)))
        (`GameplayStatics.PlaySound2D` "/Game/MusicAndSound/powerup_Cue.powerup_Cue" 1.0 1.0 0.0 null null)
        (`self.K2_DestroyActor`)))))

(fn `UserConstructionScript`)