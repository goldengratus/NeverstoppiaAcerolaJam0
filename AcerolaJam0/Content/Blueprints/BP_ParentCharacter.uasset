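; Base character shared by player and AI, built around a dash attack that launches it forward and sphere-traces for damage to the opposing side.
; Each roll starts a cooldown timer and velocity polling that returns it to Idle and turns AI toward the player.
; Hits apply knockback and material flash; death ragdolls the body and drops a power-up.
; Power-ups raise stats, while supers add timed attacks, healing, dash-bound magic circles or size.
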(event `Shoot Projectiles`
  (bind (_returnvalue_location _returnvalue_rotation) (`KismetMathLibrary.BreakTransform` (`SceneComponent.K2_GetComponentToWorld` (`self.Arrow1`))))
  (`self.DeadCheck`
    (:`Alive`
      (`|SpawnActorFromClass` "/Game/Blueprints/BP_Projectile.BP_Projectile_C" (`KismetMathLibrary.MakeTransform` _returnvalue_location _returnvalue_rotation (`KismetMathLibrary.SelectVector` (2.0 2.0 2.0) (1.0 1.0 1.0) (`self.IsPlayerControlled`))) "Undefined" "MultiplyWithRoot" null self (`self.IsPlayerControlled`) (`KismetMathLibrary.Clamp` (/ (`self.ATK`) 2) 1 999) (`self.Initial Speed`) null))))

(event `Shoot Tornado`
  (bind (_returnvalue_location _returnvalue_rotation) (`KismetMathLibrary.BreakTransform` (`SceneComponent.K2_GetComponentToWorld` (`self.Arrow1`))))
  (`self.DeadCheck`
    (:`Alive`
      (`|SpawnActorFromClass` "/Game/Blueprints/BP_Tornado.BP_Tornado_C" (`KismetMathLibrary.MakeTransform` (`SceneComponent.GetSocketLocation` (`self.Mesh`) "root") _returnvalue_rotation (`KismetMathLibrary.SelectVector` (2.0 2.0 2.0) (1.0 1.0 1.0) (`self.IsPlayerControlled`))) "Undefined" "MultiplyWithRoot" null self (`self.IsPlayerControlled`) (`KismetMathLibrary.Clamp` (/ (`self.ATK`) 2) 1 999) (+ (`self.Initial Speed`) 100.0) null))))

(event `self.ReceiveBeginPlay`
  (bind _push_power (`self.Push Power`))
  (`self.Start Rolling`)
  (set `self.Push Power` (`KismetMathLibrary.SelectFloat` _push_power (* _push_power 0.5) (`self.IsPlayerControlled`)))
  (`self.Set Resource Bar`)
  (`self.Update Max HP` (`self.Current HP`))
  (`KismetSystemLibrary.K2_SetTimerDelegate` (`|CreateDelegate` :!event `Update Roll Bar`) 0.01 true))

(event `/Game/Interface/ParentChar_INT.HP-Damage`
  (params (`ATK-Value` :type Integer) (`Push Power` :type "Vector Structure") (Atker :type "Actor Object Reference"))
  (`self.DeadCheck`
    (:`Alive`
      (`self.LaunchCharacter` `Push Power`)
      (bind _current_hp_output (`self.Change HP` (* `ATK-Value` -1)))
      (`self.Reusable SVFX` "/Game/MusicAndSound/boom_Cue.boom_Cue" "/Game/FXVarietyPack/Particles/P_ky_hit2.P_ky_hit2" (`self.K2_GetActorLocation`))
      (`self.Flash HIT`)
      (if (<= _current_hp_output 0)
        (`self.Do Death THING`)
        (message `/Game/Interface/ParentChar_INT.KilledSomething` Atker)))))

(event `Reusable SVFX`
  (params (Sound :type "SoundBase Object Reference") (EmitterTemplate :type "ParticleSystem Object Reference") (Location :type "Vector Structure") (Rotation :type "Rotator Structure"))
  (`GameplayStatics.PlaySoundAtLocation` Sound Location (struct) 1.0 1.0 0.0 null null null null)
  (`GameplayStatics.SpawnEmitterAtLocation` EmitterTemplate Location Rotation))

(event `Do Death THING`
  (`/Engine/EditorBlueprintResources/StandardMacros.DoOnce` false
    (:`Completed`
      (`self.ChangeState` "NewEnumerator3")
      (`PrimitiveComponent.SetCollisionResponseToChannel` (`self.CapsuleComponent`) "ECC_Pawn" "ECR_Ignore")
      (`SceneComponent.SetVisibility` (`self.ResourceBar`) false false)
      (`SceneComponent.SetVisibility` (`self.Arrow1`) false false)
      (`PrimitiveComponent.SetSimulatePhysics` (`self.Mesh`) true)
      (`|SpawnActorFromClass` "/Game/Blueprints/BP_PowerUp.BP_PowerUp_C" (`KismetMathLibrary.MakeTransform` (`self.K2_GetActorLocation`)) "Undefined" "MultiplyWithRoot" null (`self.PowerUpToDrop`) null)
      (`self.Death Decay`))))

(event `/Game/Interface/ParentChar_INT.ChangeState`
  (params (State :type "/Game/Enums/CharStates Enum" :default "NewEnumerator0"))
  (`self.DeadCheck`
    (:`Alive`
      (bind _output_get (set `self.Current State` State))
      (switch `/Game/Enums/CharStates` _output_get
        (:`NewEnumerator0`
          _)
        (:`NewEnumerator3`
          _))
      (`KismetArrayLibrary.Array_Clear` (`self.Actors to Ignore For Current attack`)))))

(event `Death Decay`
  (`KismetSystemLibrary.Delay` 20.0)
  (`self.K2_DestroyActor`))

(event `Set Char Max Speed`
  (params (`Max Walk Speed` :type "Float (single-precision)"))
  (set `CharacterMovementComponent.MaxWalkSpeed` `Max Walk Speed` (`self.CharacterMovement`)))

(event `Check Velocity`
  (if (== (`self.GetVelocity`) (0.0 0.0 0.0))
    (`KismetSystemLibrary.Delay` 0.2)
    (`self.ChangeState` "NewEnumerator0")
    (`KismetSystemLibrary.K2_ClearAndInvalidateTimerHandle` (stale `Start Rolling` _returnvalue))
    (`self.Turn AI to player`)))

(event `Update Roll Bar`
  (`/Game/Widgets/UI_ResourceBar.Update Roll Timer` (`self.As UI Resource Bar`) (- 1.0 (`KismetMathLibrary.SafeDivide` (`KismetSystemLibrary.K2_GetTimerRemainingTimeHandle` (`self.Roll Timer`)) (`self.Roll Loop Speed`)))))

(event `Start Rolling`
  (if (`|EnumInequality` (`self.Current State`) "NewEnumerator3")
    (if (not (`NavMovementComponent.IsFalling` (`self.CharacterMovement`)))
      (`self.Grounded Dash`)
      (`self.ThrustAttack`))
    (`self.ChangeState` "NewEnumerator1")
    (bind _returnvalue (`KismetSystemLibrary.K2_SetTimerDelegate` (delegate `Check Velocity`) 0.1 true))
    (bind _returnvalue_2 (`KismetSystemLibrary.K2_SetTimerDelegate` (`|CreateDelegate` :!event `Start Rolling`) (`self.Roll Loop Speed`)))
    (set `self.Roll Timer` _returnvalue_2)))

(event `NEW JUMP STORM POWER`
  (bind _as_bp_lightning_storm (`self.As BP Lightning Storm`)
    (:`then`
      (`/Game/Blueprints/BP_LightningStorm.Increase Rotation` _as_bp_lightning_storm))
    (:`else`
      (bind _returnvalue (`|SpawnActorFromClass` "/Game/Blueprints/BP_LightningStorm.BP_LightningStorm_C" (`KismetMathLibrary.MakeTransform` (`SceneComponent.GetSocketLocation` (`self.Mesh`) "root")) "Undefined" "MultiplyWithRoot" null self (`self.IsPlayerControlled`) (`self.ATK`) 0.0 null))
      (bind _output_get (set `self.As BP Lightning Storm` _returnvalue))
      (`self.K2_AttachToActor` _output_get self "None" "SnapToTarget" "KeepWorld" "KeepWorld" true)))
  (set `/Game/Blueprints/BP_Projectile.ATK-Value` (`self.ATK`) (`self.As BP Lightning Storm`)))

(event `Turn AI to player`
  (bind (_returnvalue_roll _returnvalue_pitch _returnvalue_yaw) (`KismetMathLibrary.BreakRotator` (`KismetMathLibrary.FindLookAtRotation` (`self.K2_GetActorLocation`) (`self.K2_GetActorLocation` (`GameplayStatics.GetPlayerCharacter` 0)))))
  (if (not (`self.IsPlayerControlled`))
    (`/Engine/EditorBlueprintResources/StandardMacros.IsValid` (`GameplayStatics.GetPlayerCharacter` 0)
      (:`Is Valid`
        (`self.K2_SetActorRotation` (`KismetMathLibrary.MakeRotator` 0.0 0.0 _returnvalue_yaw))))))

(event `Set Resource Bar`
  (bind _asui_resource_bar (cast `/Game/Widgets/UI_ResourceBar` (`WidgetComponent.GetUserWidgetObject` (`self.ResourceBar`))))
  (bind _output_get (set `self.As UI Resource Bar` _asui_resource_bar))
  (set `/Game/Widgets/UI_ResourceBar.IsPlayer?` (`self.IsPlayerControlled`) _output_get)
  (`self.Update HP HUD`)
  (`self.Update Atk HUD`))

(event `Update HP HUD`
  (bind _as_ui_resource_bar (`self.As UI Resource Bar`)
    (:`then`
      (`/Game/Widgets/UI_ResourceBar.Update HP` _as_ui_resource_bar (`self.Current HP`) (`self.MAXHP`) (`self.HP COLOR`)))
    (:`else`)))

(event `Update Atk HUD`
  (bind _as_ui_resource_bar (`self.As UI Resource Bar`)
    (:`then`
      (`/Game/Widgets/UI_ResourceBar.Update Atk` _as_ui_resource_bar (`self.ATK`)))
    (:`else`)))

(event `/Game/Interface/ParentChar_INT.Give Power Up`
  (params (`Stat Type` :type "/Game/Enums/StatsEnum Enum" :default "NewEnumerator0"))
  (bind _charactermovement (`self.CharacterMovement`))
  (`self.Change HP` (`KismetMathLibrary.Clamp` (/ (`self.MAXHP`) 3) 1 9999))
  (switch `/Game/Enums/StatsEnum` `Stat Type`
    (:`NewEnumerator0`
      (`self.Update Max HP` (+ (`self.MAXHP`) 1)))
    (:`NewEnumerator1`
      (`/Engine/EditorBlueprintResources/StandardMacros.IncrementInt` (`self.ATK`)
        (:`  `
          (`self.Update Atk HUD`))))
    (:`NewEnumerator2`
      (set `self.Roll Loop Speed` (`KismetMathLibrary.FClamp` (- (`self.Roll Loop Speed`) 0.05) 0.1 999.0))
      (set `CharacterMovementComponent.MaxWalkSpeed` (+ (`MovementComponent.GetMaxSpeed` _charactermovement) 125.0) _charactermovement)
      (`/Game/Widgets/UI_ResourceBar.Extend Stamina Bar` (`self.As UI Resource Bar`)))
    (:`NewEnumerator4`
      (`self.NEW JUMP STORM POWER`))
    (:`NewEnumerator3`
      (set `self.Shoot Speed` (`KismetMathLibrary.FClamp` (- (`self.Shoot Speed`) 0.05) 0.1 999.0))
      (`KismetSystemLibrary.K2_SetTimerDelegate` (`|CreateDelegate` :!event `Shoot Projectiles`) (`KismetMathLibrary.FClamp` (`self.Shoot Speed`) 0.1 9999.0) true)
      (set `self.Initial Speed` (+ (`self.Initial Speed`) 30.0)))
    (:`NewEnumerator5`
      (if (`self.IsPlayerControlled`)
        (message `/Game/Interface/GameInstance_INT.Victory!` (`GameplayStatics.GetGameInstance`))))))

(event `/Game/Interface/ParentChar_INT.Instant Kill`
  (if (`self.IsPlayerControlled`)
    (if (`|EnumEquality` (`self.Current State`) "NewEnumerator3")
      (`/Game/Interface/ParentChar_INT.HP-Damage` (`self.Current HP`) (0.0 0.0 0.0) self :!label _label)
      (else
        (message `/Game/Interface/GameInstance_INT.Victory!` (`GameplayStatics.GetGameInstance`))))
    (else
      (goto _label))))

(event `ThrustAttack`
  (bind _returnvalue (`self.K2_GetActorLocation`))
  (`self.LaunchCharacter` (+ (* (`KismetMathLibrary.GetForwardVector` (`self.K2_GetActorRotation`)) (`self.Push Power`)) (`self.Jump Power`)))
  (`GameplayStatics.PlaySoundAtLocation` "/Game/MusicAndSound/jump_Cue.jump_Cue" (`self.K2_GetActorLocation`) (struct) 1.0 1.0 0.0 null null null null)
  (bind (_outhits _returnvalue_2) (`KismetSystemLibrary.SphereTraceMulti` _returnvalue (+ _returnvalue (* (`KismetMathLibrary.Conv_RotatorToVector` (`SceneComponent.K2_GetComponentRotation` (`self.Arrow1`))) 200.0)) (`CapsuleComponent.CapsuleRadius` (`self.CapsuleComponent`)) "TraceTypeQuery1"))
  (`self.Damage Collision With Traces` _outhits _returnvalue_2))

(event `/Game/Interface/ParentChar_INT.KilledSomething`
  (`self.ThrustAttack`)
  (`self.Killed Something`))

(event `AOE Power`
  (bind _returnvalue (`self.K2_GetActorLocation`))
  (`self.DeadCheck`
    (:`Alive`
      (`self.Reusable SVFX` "/Game/MusicAndSound/explosion_Cue.explosion_Cue" "/Game/FXVarietyPack/Particles/P_ky_explosion.P_ky_explosion" _returnvalue)
      (bind (_outhits _returnvalue_2) (`KismetSystemLibrary.SphereTraceMulti` _returnvalue (+ _returnvalue (1.0 1.0 1.0)) (`self.Radius`) "TraceTypeQuery1"))
      (`self.Damage Collision With Traces` _outhits _returnvalue_2))))

(event `Forward Beam Power`
  (bind _returnvalue (`self.K2_GetActorLocation`))
  (bind _returnvalue_2 (`SceneComponent.K2_GetComponentRotation` (`self.Arrow1`)))
  (`self.DeadCheck`
    (:`Alive`
      (`self.Reusable SVFX` "/Game/MusicAndSound/laser_Cue.laser_Cue" "/Game/FXVarietyPack/Particles/P_ky_laser01.P_ky_laser01" _returnvalue (`KismetMathLibrary.MakeRotator` (.roll _returnvalue_2) (+ (.pitch _returnvalue_2) -90.0) (.yaw _returnvalue_2)))
      (bind (_outhits _returnvalue_3) (`KismetSystemLibrary.SphereTraceMulti` _returnvalue (+ _returnvalue (* (`KismetMathLibrary.Conv_RotatorToVector` _returnvalue_2) 1000.0)) 200.0 "TraceTypeQuery1"))
      (`self.Damage Collision With Traces` _outhits _returnvalue_3))))

(event `/Game/Interface/ParentChar_INT.Activate Super`
  (params (`Super Type` :type "/Game/Enums/SupersEnum Enum" :default "NewEnumerator0"))
  (bind _tornado_timer (`self.Tornado Timer`))
  (bind _explosion_timer (`self.Explosion Timer`))
  (bind _capsulecomponent (`self.CapsuleComponent`))
  (bind _beam_timer (`self.Beam Timer`))
  (`/Game/Widgets/UI_ResourceBar.Add Super Power Indicator` (`self.As UI Resource Bar`) `Super Type`)
  (`self.ThrustAttack`)
  (switch `/Game/Enums/SupersEnum` `Super Type`
    (:`NewEnumerator0`
      (`KismetSystemLibrary.K2_SetTimerDelegate` (`|CreateDelegate` :!event `AOE Power`) _explosion_timer true)
      (set `self.Explosion Timer` (`KismetMathLibrary.FClamp` (- _explosion_timer 0.5) 1.0 999.0)))
    (:`NewEnumerator1`
      (`KismetSystemLibrary.K2_SetTimerDelegate` (`|CreateDelegate` :!event `Forward Beam Power`) _beam_timer true)
      (set `self.Beam Timer` (`KismetMathLibrary.FClamp` (- _beam_timer 1.0) 1.0 999.0)))
    (:`NewEnumerator2`
      (`KismetSystemLibrary.K2_SetTimerDelegate` (`|CreateDelegate` :!event `Shoot Tornado`) _tornado_timer true)
      (set `self.Tornado Timer` (`KismetMathLibrary.FClamp` (- _tornado_timer 1.0) 1.0 9999.0)))
    (:`NewEnumerator3`
      (add `self.Grounded Dash` (delegate `Magic Circle Power`)))
    (:`NewEnumerator4`
      (`KismetSystemLibrary.K2_SetTimerDelegate` (`|CreateDelegate` :!event `Heal Over Time Power`) 8.0 true)
      (`/Engine/EditorBlueprintResources/StandardMacros.IncrementInt` (`self.Heal Passive Amount`)))
    (:`NewEnumerator5`
      (`self.SetActorScale3D` (+ (`self.GetActorScale3D`) (1.0 1.0 1.0)))
      (`CapsuleComponent.SetCapsuleRadius` _capsulecomponent (+ (`CapsuleComponent.CapsuleRadius` _capsulecomponent) 34.0) true))))

(event `Heal Over Time Power`
  (bind _returnvalue (`SceneComponent.GetSocketLocation` (`self.Mesh`) "root"))
  (`self.Change HP` (+ (`self.Heal Passive Amount`) (/ (`self.MAXHP`) 2)))
  (`GameplayStatics.PlaySoundAtLocation` "/Game/MusicAndSound/heal_Cue.heal_Cue" _returnvalue (struct) 1.0 1.0 0.0 null null null null)
  (bind _returnvalue_2 (`GameplayStatics.SpawnEmitterAtLocation` "/Game/FXVarietyPack/Particles/P_ky_healAura.P_ky_healAura" _returnvalue))
  (`KismetSystemLibrary.Delay` 2.0)
  (`ActorComponent.Deactivate` _returnvalue_2))

(event `Magic Circle Power`
  (`/Engine/EditorBlueprintResources/StandardMacros.FlipFlop`
    (:`A`
      (`self.DeadCheck`
        (:`Alive`
          (`|SpawnActorFromClass` "/Game/Blueprints/BP_AOEthatsActuallyProj.BP_AOEthatsActuallyProj_C" (`KismetMathLibrary.MakeTransform` (`SceneComponent.GetSocketLocation` (`self.Mesh`) "root")) "Undefined" "MultiplyWithRoot" null self (`self.IsPlayerControlled`) (`KismetMathLibrary.Clamp` (/ (`self.ATK`) 3) 3 999) 0.0 null))))))

(event `Flash HIT`
  (`self.Default Mesh Material`
    (:`then`
      _)
    (:`else`
      (set `self.Default Mesh Material` (`PrimitiveComponent.GetMaterial` (`self.Mesh`) 0))))
  (bind _counter (`/Engine/EditorBlueprintResources/StandardMacros.Do N` 2 :!label _label_2)
    (:`Exit`
      (`PrimitiveComponent.SetMaterial` (`self.Mesh`) 0 "/Game/Mats/MI_Chars7.MI_Chars7")
      (`KismetSystemLibrary.Delay` 0.1)
      (`PrimitiveComponent.SetMaterial` (`self.Mesh`) 0 (`self.Default Mesh Material`))
      (if (== _counter 2)
        (goto _label_2 :!via `Reset`)
        (else
          (goto _label_2))))))

(fn `Change HP`
  (params (`Value Added to HP` :type Integer))
  (returns (`Current HP output` :type Integer))
  (bind _output_get (set `self.Current HP` (`KismetMathLibrary.Clamp` (+ (`self.Current HP`) `Value Added to HP`) 0 (select `bool` (`self.IsPlayerControlled`) :`false` 999 :`true` (`self.MAXHP`)))))
  (`self.Update HP HUD`)
  (return _output_get))

(fn `Deal Damage?`
  (params (`Target Hit` :type "Actor Object Reference") (`Is Self Player?` :type Boolean))
  (returns (`Deal Damage?` :type Boolean))
  (bind _is_player (message `/Game/Interface/ParentChar_INT.Return is Player` `Target Hit`))
  (if (== _is_player `Is Self Player?`)
    (return false)
    (else
      (return true))))

(fn `Return is Character`
  (returns (`Character?` :type Boolean))
  (return true))

(fn `Return is Player`
  (returns (`Is Player` :type Boolean))
  (return (`self.IsPlayerControlled`)))

(fn `Return Stats`
  (returns (HP :type Integer) (ATK :type Integer) (`Roll Loop Speed` :type "Float (double-precision)"))
  (return (`self.MAXHP`) (`self.ATK`) (`self.Roll Loop Speed`)))

(fn `Update Max HP`
  (params (MAXHP :type Integer))
  (set `self.MAXHP` MAXHP)
  (`self.Update HP HUD`))

(fn `UserConstructionScript`)